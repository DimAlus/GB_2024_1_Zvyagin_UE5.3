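; Laser projectile Blueprint that sizes its beam visual from the Radius value in its Data.
; InitializeAfter runs the parent logic, then sets the Z scale of two cylinder components to Radius divided by 100, so Radius acts as beam length.
; Each cylinder is moved along X by half the Radius, which makes the beam extend forward from the actor origin instead of being centered on it.
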(event `self.InitializeAfter`
  (bind (_data_speed _data_gravity _data_despawntime _data_isradial _data_radius) (break `ProjectileInitializer` (`self.data`)))
  (bind _cylinder1 (`self.Cylinder1`))
  (bind _cylinder (`self.Cylinder`))
  (bind (_data_speed_2 _data_gravity_2 _data_despawntime_2 _data_isradial_2 _data_radius_2) (break `ProjectileInitializer` (`self.data`)))
  (bind (_relativescale3d_x _relativescale3d_y) (`KismetMathLibrary.BreakVector` (`SceneComponent.RelativeScale3D` _cylinder)))
  (bind (_relativelocation_x _relativelocation_y _relativelocation_z) (`KismetMathLibrary.BreakVector` (`SceneComponent.RelativeLocation` _cylinder1)))
  (bind (_relativescale3d_x_2 _relativescale3d_y_2) (`KismetMathLibrary.BreakVector` (`SceneComponent.RelativeScale3D` _cylinder1)))
  (bind (_relativelocation_x_2 _relativelocation_y_2 _relativelocation_z_2) (`KismetMathLibrary.BreakVector` (`SceneComponent.RelativeLocation` _cylinder)))
  (`parent.InitializeAfter`)
  (`SceneComponent.SetRelativeScale3D` _cylinder (`KismetMathLibrary.MakeVector` _relativescale3d_x _relativescale3d_y (/ _data_radius_2 100.0)))
  (`SceneComponent.K2_SetRelativeLocation` _cylinder (`KismetMathLibrary.MakeVector` (/ _data_radius_2 2.0) _relativelocation_y_2 _relativelocation_z_2) false false)
  (`SceneComponent.SetRelativeScale3D` _cylinder1 (`KismetMathLibrary.MakeVector` _relativescale3d_x_2 _relativescale3d_y_2 (/ _data_radius 100.0)))
  (`SceneComponent.K2_SetRelativeLocation` _cylinder1 (`KismetMathLibrary.MakeVector` (/ _data_radius 2.0) _relativelocation_y _relativelocation_z) false false))

(fn `UserConstructionScript`)